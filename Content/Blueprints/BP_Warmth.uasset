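; BP_Warmth is a fire with a health pool that is worn down by damage and by nearby enemies.
; On BeginPlay and about every ten seconds, via a Delay on Tick, it scans all BP_Enemy actors and loses health for each within a short horizontal radius.
; It destroys itself when health runs out.
; The steam and spark particle activations are left unwired.
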(event `self.ReceiveBeginPlay`
  (`self.CheckFireSide`))

(event `self.ReceiveTick`
  (params (DeltaSeconds :type "Float (single-precision)"))
  (`KismetSystemLibrary.Delay` 10.0)
  (`self.CheckFireSide`))

(event `self.ReceiveAnyDamage`
  (params (Damage :type "Float (single-precision)") (DamageType :type "DamageType Object Reference") (InstigatedBy :type "Controller Object Reference") (DamageCauser :type "Actor Object Reference"))
  (set `self.FireHealth` (- (`self.FireHealth`) Damage))
  (if (<= (`self.FireHealth`) 0.0)
    (`self.K2_DestroyActor`)))

(event `CheckFireSide`
  (bind _outactors (`GameplayStatics.GetAllActorsOfClass` "/Game/Blueprints/BP_Enemy.BP_Enemy_C"))
  (for _array_element _outactors
    (if (< (`self.GetHorizontalDistanceTo` _array_element self) 50.0)
      (set `self.FireHealth` (- (`self.FireHealth`) 10.0))))
  (if (<= (`self.FireHealth`) 0.0)
    (`self.K2_DestroyActor`)))

(fn `UserConstructionScript`)