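; BP_Player is the player character, with Enhanced Input movement, camera look, punch and kick attacks, and health.
; Attack montages use notifies to sphere-trace pawns ahead of AttackTracePos and apply damage, with the kick reaching farther and hitting harder.
; IsPunching, IsKicking and IsHugging act as ready flags, false during playback.
; Damage lowers Health and plays NoHug_Montage, whose notify disables input and ragdolls the mesh at zero health.
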(event `self.ReceiveBeginPlay`
  ;[0.1875 0.1875 0.1875] Input
  (`EnhancedInputSubsystemInterface.AddMappingContext` (pcsubsystem `EnhancedInputLocalPlayerSubsystem` (`GameplayStatics.GetPlayerController` 0)) "/Game/Input/IMC_PlayerInput.IMC_PlayerInput" 0 (struct)))

(event `EnhancedInput|/Game/Input/IA_Move`
  (params (ActionValue :type "Vector2D Structure") (ElapsedSeconds :type "Float (double-precision)") (TriggeredSeconds :type "Float (double-precision)") (InputAction :type "InputAction Object Reference" :default "/Game/Input/IA_Move.IA_Move"))
  (bind (_returnvalue_roll _returnvalue_pitch _returnvalue_yaw) (`KismetMathLibrary.BreakRotator` (`self.GetControlRotation`)))
  (bind (_returnvalue_roll_2 _returnvalue_pitch_2 _returnvalue_yaw_2) (`KismetMathLibrary.BreakRotator` (`self.GetControlRotation`)))
  ;[0.1875 0.1875 0.1875] Movement
  (:`Triggered`
    (`self.AddMovementInput` (`KismetMathLibrary.GetRightVector` (`KismetMathLibrary.MakeRotator` _returnvalue_roll_2 0.0 _returnvalue_yaw_2)) ActionValue_X)
    (`self.AddMovementInput` (`KismetMathLibrary.GetForwardVector` (`KismetMathLibrary.MakeRotator` _returnvalue_roll 0.0 _returnvalue_yaw)) ActionValue_Y)))

(event `EnhancedInput|/Game/Input/IA_View`
  (params (ActionValue :type "Vector2D Structure") (ElapsedSeconds :type "Float (double-precision)") (TriggeredSeconds :type "Float (double-precision)") (InputAction :type "InputAction Object Reference" :default "/Game/Input/IA_View.IA_View"))
  ;[0.1875 0.1875 0.1875] Movement
  (:`Triggered`
    (`self.AddControllerYawInput` ActionValue_X)
    (`self.AddControllerPitchInput` (* ActionValue_Y -1.0))))

(event `EnhancedInput|/Game/Input/IA_Punch`
  (params (ActionValue :type Boolean) (ElapsedSeconds :type "Float (double-precision)") (TriggeredSeconds :type "Float (double-precision)") (InputAction :type "InputAction Object Reference" :default "/Game/Input/IA_Punch.IA_Punch"))
  (bind _attacktracepos (`self.AttackTracePos`))
  (bind _returnvalue (`SceneComponent.K2_GetComponentLocation` _attacktracepos))
  ;[0.1875 0.1875 0.1875] Action
  (:`Started`
    (if (`self.IsPunching`)
      (`|PlayMontage` (`self.Mesh`) "/Game/Characters/Mannequins/Animations/Manny/Punch_Montage.Punch_Montage"
        (:`then`
          (set `self.IsPunching` false))
        (:`OnCompleted`
          (set `self.IsPunching` true))
        (:`OnInterrupted`
          (set `self.IsPunching` true))
        (:`OnNotifyBegin`
          (bind _outhit (`KismetSystemLibrary.SphereTraceSingleForObjects` :`Start` _returnvalue :`End` (+ _returnvalue (* (`SceneComponent.GetForwardVector` _attacktracepos) 100.0)) :`Radius` 25.0 :`ObjectTypes` (`|MakeArray` "ObjectTypeQuery3" :!type "EObjectTypeQuery Enum") :`DrawDebugType` "ForDuration"))
          (if true
            (`GameplayStatics.ApplyDamage` (`.HitActor` (`GameplayStatics.BreakHitResult` _outhit)) 10.0)))))))

(event `EnhancedInput|/Game/Input/IA_Kick`
  (params (ActionValue :type Boolean) (ElapsedSeconds :type "Float (double-precision)") (TriggeredSeconds :type "Float (double-precision)") (InputAction :type "InputAction Object Reference" :default "/Game/Input/IA_Kick.IA_Kick"))
  (bind _attacktracepos (`self.AttackTracePos`))
  (bind _returnvalue (`SceneComponent.K2_GetComponentLocation` _attacktracepos))
  ;[0.1875 0.1875 0.1875] Action
  (:`Started`
    (if (`self.isKicking`)
      (`|PlayMontage` (`self.Mesh`) "/Game/Characters/Mannequins/Animations/Manny/Kick_Montage.Kick_Montage"
        (:`then`
          (set `self.isKicking` false))
        (:`OnCompleted`
          (set `self.isKicking` true))
        (:`OnInterrupted`
          (set `self.isKicking` true))
        (:`OnNotifyBegin`
          (bind _outhit (`KismetSystemLibrary.SphereTraceSingleForObjects` :`Start` _returnvalue :`End` (+ _returnvalue (* (`SceneComponent.GetForwardVector` _attacktracepos) 200.0)) :`Radius` 25.0 :`ObjectTypes` (`|MakeArray` "ObjectTypeQuery3" :!type "EObjectTypeQuery Enum") :`DrawDebugType` "ForDuration"))
          (if true
            (`GameplayStatics.ApplyDamage` (`.HitActor` (`GameplayStatics.BreakHitResult` _outhit)) 50.0)))))))

(event `self.ReceiveAnyDamage`
  (params (Damage :type "Float (single-precision)") (DamageType :type "DamageType Object Reference") (InstigatedBy :type "Controller Object Reference") (DamageCauser :type "Actor Object Reference"))
  (set `self.Health` (- (`self.Health`) Damage))
  (if (`self.IsHugging`)
    (`|PlayMontage` (`self.Mesh`) "/Game/Characters/Mannequins/Animations/Manny/NoHug_Montage.NoHug_Montage"
      (:`then`
        ;[0.1875 0.1875 0.1875] Action
        (set `self.IsHugging` false))
      (:`OnCompleted`
        (set `self.IsHugging` true))
      (:`OnInterrupted`
        (set `self.IsHugging` true))
      (:`OnNotifyBegin`
        (if (<= (`self.Health`) 0.0)
          (`self.DisableInput` null)
          (`PrimitiveComponent.SetSimulatePhysics` (`self.Mesh`) true))))))

(fn `UserConstructionScript`)