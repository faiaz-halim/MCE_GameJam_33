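; BP_Enemy is an enemy character that chases player 0 from BeginPlay and attacks with a hug montage.
; On reaching the player it plays the montage, whose notify sphere-traces from AttackTracePos to apply damage, then resumes chasing when the montage ends.
; Incoming damage lowers Health, launching it backward, or ragdolling the mesh and disabling hugging at zero.
; A looping random-point Roam event is defined but never called here.
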(event `self.ReceiveBeginPlay`
  (`self.ChasePlayer`))

(event `ChasePlayer`
  (bind _attacktracepos (`self.AttackTracePos`))
  (bind _returnvalue (`SceneComponent.K2_GetComponentLocation` _attacktracepos))
  ;[0.1875 0.1875 0.1875] Chase Player
  (`|AIMoveTo` self (0.0 0.0 0.0) (`GameplayStatics.GetPlayerCharacter` 0)
    (:`OnSuccess`
      (if (`self.IsHugging`)
        (`|PlayMontage` (`self.Mesh`) "/Game/Characters/Mannequins/Animations/Manny/Hug_Montage.Hug_Montage"
          (:`then`
            (set `self.IsHugging` false))
          (:`OnCompleted`
            (set `self.IsHugging` true)
            (`self.ChasePlayer` :!label _label))
          (:`OnInterrupted`
            (set `self.IsHugging` true)
            (goto _label))
          (:`OnNotifyBegin`
            (bind (_outhit _returnvalue_2) (`KismetSystemLibrary.SphereTraceSingleForObjects` :`Start` _returnvalue :`End` (+ _returnvalue (* (`SceneComponent.GetForwardVector` _attacktracepos) 100.0)) :`ObjectTypes` (`|MakeArray` "ObjectTypeQuery3" :!type "EObjectTypeQuery Enum") :`DrawDebugType` "ForDuration"))
            (if _returnvalue_2
              (`GameplayStatics.ApplyDamage` (`.HitActor` (`GameplayStatics.BreakHitResult` _outhit)) 10.0))))))))

(event `Roam`
  ;[0.1875 0.1875 0.1875] Roam
  (`|AIMoveTo` self (`NavigationSystemV1.K2_GetRandomReachablePointInRadius` (`self.K2_GetActorLocation`) 500.0 null null) null
    (:`OnSuccess`
      (`KismetSystemLibrary.Delay` 1.0)
      (`self.Roam`))))

(event `self.ReceiveAnyDamage`
  (params (Damage :type "Float (single-precision)") (DamageType :type "DamageType Object Reference") (InstigatedBy :type "Controller Object Reference") (DamageCauser :type "Actor Object Reference"))
  ;[0.1875 0.1875 0.1875] Damage System
  (set `self.Health` (- (`self.Health`) Damage))
  (if (<= (`self.Health`) 0.0)
    (`PrimitiveComponent.SetSimulatePhysics` (`self.Mesh`) true)
    (set `self.IsHugging` false)
    (else
      (`self.LaunchCharacter` (+ (* (`self.GetActorForwardVector`) -200.0) (* (`self.GetActorUpVector`) 100.0))))))

(fn `UserConstructionScript`)