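; BP_WaveSpawn is a wave spawner that creates BP_Enemy actors at its own transform, starting the first wave on BeginPlay.
; SpawnWave increments CurrentWave and uses the matching entry in the Waves map's values as the enemy count.
; CheckforEnemies, which nothing in this file calls, waits briefly and starts the next wave when no BP_Enemy actors remain.
; No bounds check guards against running past the last wave.
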(event `self.ReceiveBeginPlay`
  (`self.Spawn Wave`))

(event `Spawn Wave`
  (`/Engine/EditorBlueprintResources/StandardMacros.IncrementInt` (`self.Current Wave`)
    (:`  `
      (bind _values (`BlueprintMapLibrary.Map_Values` (`self.Waves`)))
      (for _ (range (+ (`|GetArrayItem` _values (- (`self.Current Wave`) 1)) 1))
        (`|SpawnActorFromClass` "/Game/Blueprints/BP_Enemy.BP_Enemy_C" (`self.GetTransform`) "AdjustIfPossibleButAlwaysSpawn" "MultiplyWithRoot" null null)))))

(event `Check for Enemies`
  (`KismetSystemLibrary.Delay` 0.2)
  (bind _outactors (`GameplayStatics.GetAllActorsOfClass` "/Game/Blueprints/BP_Enemy.BP_Enemy_C"))
  (if (== (`KismetArrayLibrary.Array_Length` _outactors) 0)
    (`self.Spawn Wave`)))

(fn `UserConstructionScript`)